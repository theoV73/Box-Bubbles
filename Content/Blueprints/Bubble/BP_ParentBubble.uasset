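; Parent bubble actor that affects characters touching it according to its type: Tapioka, Soap, Glass, Gum or Water.
; SetBubbleIndex, called with Glass on BeginPlay, updates material, idle Niagara effect and box collision (overlap for Tapioka and Water, block otherwise).
; Box overlap launches characters upward for Tapioka or spawns splashes for Soap and Water.
; Box hit temporarily boosts speed for Soap or lowers speed and gravity for Gum, then restores hardcoded values.
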(event OnComponentBeginOverlap(Box)
  (params (OverlappedComponent :type Primitive%20Component%20Object%20Reference) (OtherActor :type Actor%20Object%20Reference) (OtherComp :type Primitive%20Component%20Object%20Reference) (OtherBodyIndex :type Integer) (bFromSweep :type Boolean) (SweepResult :type Hit%20Result%20Structure%20%28by%20ref%29))
  (switch Utilities|FlowControl|Switch|SwitchonEN_Bubble (Variables|Default|GetBubbleIndex)
    (:NewEnumerator0
      (bind _ascharacter (Utilities|Casting|CastToCharacter OtherActor))
      (Character|LaunchCharacter _ascharacter "0.000000,0.000000,1150.000000" false true))
    (:NewEnumerator1
      (Utilities|Casting|CastToCharacter OtherActor)
      (Niagara|SpawnSystematLocation "/Game/VFX/NiagaraSystem/CollisionEffect/NS_SoapSplash.NS_SoapSplash" (Transformation|GetWorldLocation (Variables|Default|GetBox))))
    (:NewEnumerator4
      (Utilities|Casting|CastToCharacter OtherActor)
      (Niagara|SpawnSystematLocation "/Game/VFX/NiagaraSystem/CollisionEffect/NS_WaterSplash.NS_WaterSplash" (Transformation|GetWorldLocation (Variables|Default|GetSphereMesh))))))

(event OnComponentHit(Box)
  (params (HitComponent :type Primitive%20Component%20Object%20Reference) (OtherActor :type Actor%20Object%20Reference) (OtherComp :type Primitive%20Component%20Object%20Reference) (NormalImpulse :type Vector :default "0, 0, 0") (Hit :type Hit%20Result%20Structure%20%28by%20ref%29))
  (switch Utilities|FlowControl|Switch|SwitchonEN_Bubble (Variables|Default|GetBubbleIndex)
    (:NewEnumerator1
      (bind _ascharacter (Utilities|Casting|CastToCharacter OtherActor))
      (Variables|/Script/Engine.CharacterMovementComponent|SetMaxWalkSpeed (Variables|/Script/Engine.Character|GetCharacterMovement _ascharacter) 1.2e+03)
      (Utilities|FlowControl|Delay 3.0)
      (Variables|/Script/Engine.CharacterMovementComponent|SetMaxWalkSpeed (Variables|/Script/Engine.Character|GetCharacterMovement _ascharacter) 5e+02))
    (:NewEnumerator3
      (bind _ascharacter_2 (Utilities|Casting|CastToCharacter OtherActor))
      (Variables|/Script/Engine.CharacterMovementComponent|SetMaxWalkSpeed (Variables|/Script/Engine.Character|GetCharacterMovement _ascharacter_2) 2.5e+02)
      (Variables|/Script/Engine.CharacterMovementComponent|SetGravityScale (Variables|/Script/Engine.Character|GetCharacterMovement _ascharacter_2) 0.5)
      (Character|LaunchCharacter _ascharacter_2 "0, 0, 0" false true)
      (Utilities|FlowControl|Delay 3.0)
      (Variables|/Script/Engine.CharacterMovementComponent|SetMaxWalkSpeed (Variables|/Script/Engine.Character|GetCharacterMovement _ascharacter_2) 5e+02)
      (Variables|/Script/Engine.CharacterMovementComponent|SetGravityScale (Variables|/Script/Engine.Character|GetCharacterMovement _ascharacter_2) 1.75))))

(event EventBeginPlay
  (CallFunction|SetBubbleIndex "NewEnumerator2"))

(event Collision|EventActorBeginOverlap
  (params (OtherActor :type Actor%20Object%20Reference)))

(event EventTick
  (params (DeltaSeconds :type Float%20%28single-precision%29)))

(fn ConstructionScript)

(fn SetBubbleEsthetic
  (bind _bubbleindex (Variables|Default|GetBubbleIndex))
  (Rendering|Material|SetMaterial (Variables|Default|GetSphereMesh) 0 (Utilities|Select :Index _bubbleindex :NewEnumerator0 "/Game/Material/M_Tapioca02.M_Tapioca02" :NewEnumerator1 "/Game/Material/M_SoapBubble.M_SoapBubble" :NewEnumerator2 "/Game/Material/M_Glass.M_Glass" :NewEnumerator3 "/Game/Material/M_ChewingGum.M_ChewingGum" :NewEnumerator4 "/Game/Material/M_WaterBubble03.M_WaterBubble03"))
  (Utilities|IsValid (Variables|Default|GetNS_IdleBubbleRef)
    (:Is%20Valid
      (Components|DestroyComponent (Variables|Default|GetNS_IdleBubbleRef)))
    (:Is%20Not%20Valid
      _))
  (switch Utilities|FlowControl|Switch|SwitchonEN_Bubble _bubbleindex
    (:NewEnumerator1
      (bind _returnvalue (Niagara|SpawnSystematLocation 0 (Transformation|GetWorldLocation (Variables|Default|GetSphereMesh))))
      (Variables|Default|SetNS_IdleBubbleRef _returnvalue))
    (:NewEnumerator4
      (bind _returnvalue_2 (Niagara|SpawnSystematLocation "/Game/VFX/NiagaraSystem/BubbleIdle/NS_WaterBubbleIdle.NS_WaterBubbleIdle" (Transformation|GetWorldLocation (Variables|Default|GetSphereMesh)) "0, 0, 0" "1.000000,1.000000,1.000000" false))
      (Variables|Default|SetNS_IdleBubbleRef _returnvalue_2))))

(fn SetBubbleIndex
  (params (BubbleIndex :type EN_Bubble%20Enum :default "NewEnumerator0"))
  (Variables|Default|SetBubbleIndex BubbleIndex)
  (CallFunction|SetBubbleEsthetic)
  (CallFunction|SetBubbleCollision))

(fn SetBubbleCollision
  (switch Utilities|FlowControl|Switch|SwitchonEN_Bubble (Variables|Default|GetBubbleIndex)
    (:NewEnumerator0
      (Collision|SetCollisionResponsetoAllChannels (Variables|Default|GetBox) "ECR_Overlap"))
    (:NewEnumerator1
      (Collision|SetCollisionResponsetoAllChannels (Variables|Default|GetBox) "ECR_Block" :!label _label))
    (:NewEnumerator2
      (goto _label))
    (:NewEnumerator3
      (goto _label))
    (:NewEnumerator4
      (Collision|SetCollisionResponsetoAllChannels (Variables|Default|GetBox) "ECR_Overlap"))))