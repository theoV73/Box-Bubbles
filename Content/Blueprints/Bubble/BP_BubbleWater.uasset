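; Water bubble actor that changes the third-person character's gravity while it is inside the collision sphere.
; Sphere begin overlap sets the character movement's gravity scale to the bubble's GravityScale variable, and end overlap resets it to normal rather than restoring the prior value.
; Both crossings spawn a Niagara water splash using the character's last movement update location.
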(event OnComponentBeginOverlap(SphereCollision)
  (params (OverlappedComponent :type Primitive%20Component%20Object%20Reference) (OtherActor :type Actor%20Object%20Reference) (OtherComp :type Primitive%20Component%20Object%20Reference) (OtherBodyIndex :type Integer) (bFromSweep :type Boolean) (SweepResult :type Hit%20Result%20Structure%20%28by%20ref%29))
  (bind _asbp_third_person_character (Utilities|Casting|CastToBP_ThirdPersonCharacter OtherActor))
  (Variables|/Script/Engine.CharacterMovementComponent|SetGravityScale (Variables|/Script/Engine.Character|GetCharacterMovement _asbp_third_person_character) (Variables|Default|GetGravityScale))
  (Niagara|SpawnSystemAttached "/Game/VFX/NiagaraSystem/NS_WaterSplash.NS_WaterSplash" 0 "None" (Class|CharacterMovementComponent|GetLastUpdateLocation (Variables|/Script/Engine.Character|GetCharacterMovement _asbp_third_person_character)) "0, 0, 0" "KeepRelativeOffset" false))

(event OnComponentEndOverlap(SphereCollision)
  (params (OverlappedComponent :type Primitive%20Component%20Object%20Reference) (OtherActor :type Actor%20Object%20Reference) (OtherComp :type Primitive%20Component%20Object%20Reference) (OtherBodyIndex :type Integer))
  (bind _asbp_third_person_character (Utilities|Casting|CastToBP_ThirdPersonCharacter OtherActor))
  (Variables|/Script/Engine.CharacterMovementComponent|SetGravityScale (Variables|/Script/Engine.Character|GetCharacterMovement _asbp_third_person_character) 1.0)
  (Niagara|SpawnSystemAttached "/Game/VFX/NiagaraSystem/NS_WaterSplash.NS_WaterSplash" 0 "None" (Class|CharacterMovementComponent|GetLastUpdateLocation (Variables|/Script/Engine.Character|GetCharacterMovement _asbp_third_person_character)) "0, 0, 0" "KeepRelativeOffset" false))

(event EventBeginPlay)

(event Collision|EventActorBeginOverlap
  (params (OtherActor :type Actor%20Object%20Reference)))

(fn ConstructionScript)