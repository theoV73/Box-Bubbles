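; Bubble actor that switches its appearance between five bubble types: glass, water, tapioca, soap and gum.
; ChangesBubbles ignores an unchanged value, otherwise stores it and uses an if chain to show the matching component and hide the other four.
; Each switch prints a debug label, with the gum and tapioca labels swapped relative to the components shown.
; The event graph is empty, and an unconnected snippet setting third-person character gravity never runs.
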(event EventBeginPlay)

(event Collision|EventActorBeginOverlap
  (params (OtherActor :type Actor%20Object%20Reference)))

(fn ConstructionScript)

(fn ChangesBubbles
  (params (NewBubbles :type Integer64%20%28by%20ref%29))
  (bind _bp_bubleglass (Variables|Default|GetBP_BubleGlass))
  (bind _bp_bubblewater (Variables|Default|GetBP_BubbleWater))
  (bind _bp_bubbletapioka (Variables|Default|GetBP_BubbleTapioka))
  (bind _bp_bubblesoap (Variables|Default|GetBP_BubbleSoap))
  (bind _bp_bubblegum (Variables|Default|GetBP_BubbleGum))
  (if (not (== NewBubbles (Variables|Default|GetValuesBubble)))
    (bind _output_get (Variables|Default|SetValuesBubble NewBubbles))
    (if (== _output_get 0)
      (Rendering|SetVisibility _bp_bubleglass true true)
      (Rendering|SetVisibility _bp_bubblewater false true)
      (Rendering|SetVisibility _bp_bubbletapioka false true)
      (Rendering|SetVisibility _bp_bubblesoap false true)
      (Rendering|SetVisibility _bp_bubblegum false true)
      (Development|PrintText "Bubble = Glass")
      (elif (== _output_get 1)
        (Rendering|SetVisibility _bp_bubleglass false true)
        (Rendering|SetVisibility _bp_bubblewater true true)
        (Rendering|SetVisibility _bp_bubbletapioka false true)
        (Rendering|SetVisibility _bp_bubblesoap false true)
        (Rendering|SetVisibility _bp_bubblegum false true)
        (Development|PrintText "Bubble = water")
        (elif (== _output_get 2)
          (Rendering|SetVisibility _bp_bubleglass false true)
          (Rendering|SetVisibility _bp_bubblewater false true)
          (Rendering|SetVisibility _bp_bubbletapioka true true)
          (Rendering|SetVisibility _bp_bubblesoap false true)
          (Rendering|SetVisibility _bp_bubblegum false true)
          (Development|PrintText "Bubble = gum")
          (elif (== _output_get 3)
            (Rendering|SetVisibility _bp_bubleglass false true)
            (Rendering|SetVisibility _bp_bubblewater false true)
            (Rendering|SetVisibility _bp_bubbletapioka false true)
            (Rendering|SetVisibility _bp_bubblesoap true true)
            (Rendering|SetVisibility _bp_bubblegum false true)
            (Development|PrintText "Bubble = soap")
            (elif (== _output_get 4)
              (Rendering|SetVisibility _bp_bubleglass false true)
              (Rendering|SetVisibility _bp_bubblewater false true)
              (Rendering|SetVisibility _bp_bubbletapioka false true)
              (Rendering|SetVisibility _bp_bubblesoap false true)
              (Rendering|SetVisibility _bp_bubblegum true true)
              (Development|PrintText "Bubble = tapioka"))))))))