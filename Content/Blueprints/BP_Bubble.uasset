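; Bubble actor that can appear as one of five bubble types: glass, water, gum, soap or tapioka.
; ChangesBubbles stores the given index in ValuesBubble and, through a chain of equality checks, shows the matching component and its children while hiding the other four.
; Each switch prints the chosen type as debug text.
; The event graph and construction script are empty, so switching relies on an external call.
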(event EventBeginPlay)

(event Collision|EventActorBeginOverlap
  (params (OtherActor :type Actor%20Object%20Reference)))

(fn ConstructionScript)

(fn ChangesBubbles
  (params (NewBubbles :type Integer64))
  (bind _output_get (Variables|Default|SetValuesBubble NewBubbles))
  (if (== _output_get 0)
    (Rendering|SetVisibility (Variables|Composants|GetBubbles_Glass) true true)
    (Rendering|SetVisibility (Variables|Composants|GetBubbles_Water) false true)
    (Rendering|SetVisibility (Variables|Composants|GetBubbles_Gum) false true)
    (Rendering|SetVisibility (Variables|Composants|GetBubbles_Soap) false true)
    (Rendering|SetVisibility (Variables|Composants|GetBubbles_Tapioka) false true)
    (Development|PrintText "Bubble = Glass")
    (elif (== _output_get 1)
      (Rendering|SetVisibility (Variables|Composants|GetBubbles_Glass) false true)
      (Rendering|SetVisibility (Variables|Composants|GetBubbles_Water) true true)
      (Rendering|SetVisibility (Variables|Composants|GetBubbles_Gum) false true)
      (Rendering|SetVisibility (Variables|Composants|GetBubbles_Soap) false true)
      (Rendering|SetVisibility (Variables|Composants|GetBubbles_Tapioka) false true)
      (Development|PrintText "Bubble = water")
      (elif (== _output_get 2)
        (Rendering|SetVisibility (Variables|Composants|GetBubbles_Glass) false true)
        (Rendering|SetVisibility (Variables|Composants|GetBubbles_Water) false true)
        (Rendering|SetVisibility (Variables|Composants|GetBubbles_Gum) true true)
        (Rendering|SetVisibility (Variables|Composants|GetBubbles_Soap) false true)
        (Rendering|SetVisibility (Variables|Composants|GetBubbles_Tapioka) false true)
        (Development|PrintText "Bubble = gum")
        (elif (== _output_get 3)
          (Rendering|SetVisibility (Variables|Composants|GetBubbles_Glass) false true)
          (Rendering|SetVisibility (Variables|Composants|GetBubbles_Water) false true)
          (Rendering|SetVisibility (Variables|Composants|GetBubbles_Gum) false true)
          (Rendering|SetVisibility (Variables|Composants|GetBubbles_Soap) true true)
          (Rendering|SetVisibility (Variables|Composants|GetBubbles_Tapioka) false true)
          (Development|PrintText "Bubble = soap")
          (elif (== _output_get 4)
            (Rendering|SetVisibility (Variables|Composants|GetBubbles_Glass) false true)
            (Rendering|SetVisibility (Variables|Composants|GetBubbles_Water) false true)
            (Rendering|SetVisibility (Variables|Composants|GetBubbles_Gum) false true)
            (Rendering|SetVisibility (Variables|Composants|GetBubbles_Soap) false true)
            (Rendering|SetVisibility (Variables|Composants|GetBubbles_Tapioka) true true)
            (Development|PrintText "Bubble = tapioka")))))))